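; BP_BaseWeapon is a base gun actor that provides shared hitscan and projectile firing logic.
; FireWeapon line-traces forward from the LineTrace component, ignoring itself and the player, applies damage to the hit actor and spawns blood on actors tagged "enemy".
; FireProjectile spawns a projectile at ProjectileTransform, passing it speed and damage.
; ShootWeapon and StopShooting are empty events, while PlayWeaponSound plays the weapon's sound at its location.
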(event `ShootWeapon`)

(event `StopShooting`)

(event `Play Weapon Sound`
  (`GameplayStatics.PlaySoundAtLocation` (`self.Sound`) (`self.K2_GetActorLocation`) (struct) 1.0 1.0 0.0 null null null null))

(fn `FireProjectile`
  (`|SpawnActorFromClass` (`self.Projectile`) (`SceneComponent.K2_GetComponentToWorld` (`self.ProjectileTransform`)) "Undefined" "MultiplyWithRoot" null (`self.ProjectileSpeed`) (`self.Base Damage`) null))

(fn `FireWeapon`
  (bind _returnvalue (`SceneComponent.K2_GetComponentLocation` (`self.LineTrace`)))
  (bind (_outhit _returnvalue_2) (`KismetSystemLibrary.LineTraceSingleForObjects` _returnvalue (+ _returnvalue (* (`KismetMathLibrary.GetForwardVector` (`SceneComponent.K2_GetComponentRotation` (`self.LineTrace`))) (`self.LineTraceDistance`))) (`|MakeArray` "ObjectTypeQuery1" "ObjectTypeQuery2" "ObjectTypeQuery3" :!type "EObjectTypeQuery Enum") false (`|MakeArray` self (`GameplayStatics.GetPlayerCharacter` 0) :!type "Actor Object Reference")))
  (if _returnvalue_2
    (bind (_bblockinghit _binitialoverlap _time _distance _location _impactpoint _normal _impactnormal _physmat _hitactor) (`GameplayStatics.BreakHitResult` _outhit))
    (`GameplayStatics.ApplyDamage` _hitactor (`self.Base Damage`))
    (if (`self.ActorHasTag` _hitactor "enemy")
      (`|SpawnActorFromClass` "/Game/Enemy/Blood/Blood_BP.Blood_BP_C" (`KismetMathLibrary.MakeTransform` _location) "Undefined" "MultiplyWithRoot" null null))))

(fn `UserConstructionScript`)