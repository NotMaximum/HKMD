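; BaseEnemy_BP is an enemy Blueprint that currently only debugs where the player is relative to its facing.
; Each Tick takes the arccosine of the dot product between its forward vector and the direction to the player, printing the angle in degrees.
; The sign of the right-vector dot product tells whether the player is to its left, which is also printed.
; The branch on that side test has no actions yet.
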(event `self.ReceiveTick`
  (params (DeltaSeconds :type "Float (single-precision)"))
  (bind _returnvalue (`KismetMathLibrary.Normal` (- (`self.K2_GetActorLocation` (`GameplayStatics.GetPlayerCharacter` 0)) (`self.K2_GetActorLocation`))))
  (bind _returnvalue_2 (< (`KismetMathLibrary.Dot_VectorVector` (`self.GetActorRightVector`) _returnvalue) 0.0))
  (bind _output_get (set `self.Degrees` (`KismetMathLibrary.DegAcos` (`KismetMathLibrary.Dot_VectorVector` (`self.GetActorForwardVector`) _returnvalue))))
  (`KismetSystemLibrary.PrintString` (`KismetStringLibrary.Conv_DoubleToString` _output_get) true true (struct :`G` 1.0 :`B` 0.194485 :`A` 1.0))
  (`KismetSystemLibrary.PrintString` (`KismetStringLibrary.Conv_BoolToString` _returnvalue_2))
  (if _returnvalue_2
    _))

(fn `UserConstructionScript`)