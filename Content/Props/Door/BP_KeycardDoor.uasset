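; Keycard-locked door whose KeycardDoor setting selects red, orange or blue, with the construction script assigning the matching cube material.
; On box overlap it checks the first-person character's flag for that colour, then plays a one-shot Timeline raising the cube and destroys the door after a short delay.
; The blue keycard check is disconnected, so blue doors never open.
; Each lerp starts from the cube's current height, so the rise accumulates per update.
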(event `self.Box.OnComponentBeginOverlap`
  (params (OverlappedComponent :type "PrimitiveComponent Object Reference") (OtherActor :type "Actor Object Reference") (OtherComp :type "PrimitiveComponent Object Reference") (OtherBodyIndex :type Integer) (bFromSweep :type Boolean) (SweepResult :type "HitResult Structure (by ref)"))
  (bind _cube (`self.Cube`))
  (bind (_returnvalue_x _returnvalue_y _returnvalue_z) (`KismetMathLibrary.BreakVector` (`SceneComponent.K2_GetComponentLocation` _cube)))
  (bind _asbp_first_person_character (cast `/Game/FirstPerson/Blueprints/BP_FirstPersonCharacter` OtherActor))
  (set `self.As BP First Person Character` _asbp_first_person_character)
  (switch `/Game/Props/Keys/Keycard` (`self.KeycardDoor`)
    (:`NewEnumerator0`
      (if (`/Game/FirstPerson/Blueprints/BP_FirstPersonCharacter.redkeycard?` (`self.As BP First Person Character`))
        (`/Engine/EditorBlueprintResources/StandardMacros.DoOnce` false :!label _label
          (:`Completed`
            (bind (_direction _newtrack_0) (`Timeline|Timeline`)
              (:`Update`
                (`SceneComponent.K2_SetWorldLocation` _cube (`KismetMathLibrary.MakeVector` _returnvalue_x _returnvalue_y (`KismetMathLibrary.Lerp` _returnvalue_z (+ _returnvalue_z 25.0) _newtrack_0)) false false))
              (:`Finished`
                (`KismetSystemLibrary.Delay` 0.2)
                (`self.K2_DestroyActor`)))))))
    (:`NewEnumerator1`
      (if (`/Game/FirstPerson/Blueprints/BP_FirstPersonCharacter.orangekeycard?` (`self.As BP First Person Character`))
        (goto _label)))))

(fn `UserConstructionScript`
  (switch `/Game/Props/Keys/Keycard` (`self.KeycardDoor`)
    (:`NewEnumerator0`
      (`PrimitiveComponent.SetMaterial` (`self.Cube`) 0 "/Game/Megascans/Surfaces/Paper_pblfqvp0/MI_Paper_pblfqvp0_1K.MI_Paper_pblfqvp0_1K"))
    (:`NewEnumerator1`
      (`PrimitiveComponent.SetMaterial` (`self.Cube`) 0 "/Game/Megascans/Surfaces/Orange_Metal_Sheet_ubphaenlw/MI_Orange_Metal_Sheet_ubphaenlw_1K.MI_Orange_Metal_Sheet_ubphaenlw_1K"))
    (:`NewEnumerator2`
      (`PrimitiveComponent.SetMaterial` (`self.Cube`) 0 "/Game/LevelPrototyping/Materials/MI_Solid_Blue.MI_Solid_Blue"))))