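; BP_Projectile is a pistol projectile actor that damages whatever it hits, using a Paper2D flipbook for its visuals and a projectile movement component.
; On hit it applies its damage value to the other actor, swaps to a destroyed-projectile flipbook, waits for that animation's length, then destroys itself.
; Construction script nodes that would copy the speed variable into the movement's initial and max speed are unconnected, so they never run.
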(event `self.ReceiveHit`
  (params (MyComp :type "PrimitiveComponent Object Reference") (Other :type "Actor Object Reference") (OtherComp :type "PrimitiveComponent Object Reference") (bSelfMoved :type Boolean) (HitLocation :type "Vector Structure") (HitNormal :type "Vector Structure") (NormalImpulse :type "Vector Structure") (Hit :type "HitResult Structure (by ref)"))
  (bind _paperflipbook (`self.PaperFlipbook`))
  (`GameplayStatics.ApplyDamage` Other (`self.ProjectileDamage`))
  (`PaperFlipbookComponent.SetFlipbook` _paperflipbook (`self.DestroyedProjectile`))
  (`KismetSystemLibrary.Delay` (`PaperFlipbookComponent.GetFlipbookLength` _paperflipbook))
  (`self.K2_DestroyActor`))

(fn `UserConstructionScript`)